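; Rail shooter target that slides back and forth between two waypoints and is destroyed when its health runs out.
; From BeginPlay, a FlipFlop alternately plays a timeline forward and in reverse, lerping the mesh's relative location between the left and right waypoint components.
; The timeline's Finished output calls the move event again to keep the loop going.
; ReduceHealthPoints subtracts damage and destroys the actor at zero or below.
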(event Custom|MoveToWaypoint
  (Utilities|FlowControl|FlipFlop
    (:A
      (bind _alpha (Timeline|TL_MoveToWaypoint PlayFromStart)
        (:Update
          (Transformation|SetRelativeLocation (Variables|Default|GetTargetMesh) (Math|Vector|Lerp(Vector) (Variables|/Script/Engine.SceneComponent|GetRelativeLocation (Variables|Default|GetWP_L)) (Variables|/Script/Engine.SceneComponent|GetRelativeLocation (Variables|Default|GetWP_R)) _alpha) false false))
        (:Finished
          (CallFunction|MovetoWaypoint))))
    (:B
      (Timeline|TL_MoveToWaypoint ReverseFromEnd))))

(event Custom|ReduceHealthPoints
  (params (Damage :type Float%20%28double-precision%29))
  (bind _output_get (Variables|Default|SetHealthPoints (- (Variables|Default|GetHealthPoints) Damage)))
  (if (<= _output_get 0.0)
    (Actor|DestroyActor)))

(event EventBeginPlay
  (CallFunction|MovetoWaypoint))

(event Collision|EventActorBeginOverlap
  (params (OtherActor :type Actor%20Object%20Reference)))

(event EventTick
  (params (DeltaSeconds :type Float%20%28single-precision%29)))

(fn ConstructionScript)