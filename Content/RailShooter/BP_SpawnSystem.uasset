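; Spawner for the rail shooter that periodically creates waves of BP_Target enemies ahead of the player along world X.
; On BeginPlay it caches the player character, spawns a first wave, then repeats on a looping timer set by SpawnTimer.
; Each wave spawns a random number of targets at DistanceFromPlayer from the player's current location, scattered randomly sideways and vertically.
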(event Custom|SpawnEnemies
  (for _index (range 0 (Math|Random|RandomIntegerinRange 3 (Variables|Default|GetEnemySpawnCountMax)))
    (Game|SpawnActorfromClass "/Game/RailShooter/BP_Target.BP_Target_C" (Math|Transform|MakeTransform (+ (Transformation|GetActorLocation (Variables|Default|GetPlayer)) (Math|Vector|MakeVector (Variables|Default|GetDistanceFromPlayer) (Math|Random|RandomFloatinRange -4e+02 4e+02) (Math|Random|RandomFloatinRange -5e+01 2.5e+02))) "0.000000,180.000000,0.000000" "1.000000,1.000000,1.000000") "Undefined" "MultiplyWithRoot" 0 0)))

(event EventBeginPlay
  (bind _asbp_rail_shooter_character_child (Utilities|Casting|CastToBP_RailShooterCharacter_Child (Game|GetPlayerCharacter 0)))
  (Variables|Default|SetPlayer _asbp_rail_shooter_character_child)
  (CallFunction|SpawnEnemies)
  (Utilities|Time|SetTimerbyEvent (delegate Custom|SpawnEnemies) (Variables|Default|GetSpawnTimer) true))

(event Collision|EventActorBeginOverlap
  (params (OtherActor :type Actor%20Object%20Reference)))

(event EventTick
  (params (DeltaSeconds :type Float%20%28single-precision%29)))

(fn ConstructionScript)